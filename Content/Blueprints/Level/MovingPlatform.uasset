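; Moving platform actor that shifts itself from its starting location along a timeline that starts at BeginPlay.
; It stores the initial location, then on each timeline update adds the value of one of two tracks, forward or backwards, as chosen by the MoveForward flag.
; Position is set directly without sweeping, so movement does not stop on collisions.
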(event `self.ReceiveBeginPlay`
  (set `self.Initial Position` (`self.K2_GetActorLocation`))
  (bind (_direction _move_forward _move_backwards) (`Timeline|Movement Timeline`)
    (:`Update`
      (if (`self.Move Forward`)
        (`self.K2_SetActorLocation` (+ (`self.Initial Position`) _move_forward))
        (else
          (`self.K2_SetActorLocation` (+ (`self.Initial Position`) _move_backwards)))))))

(fn `UserConstructionScript`)