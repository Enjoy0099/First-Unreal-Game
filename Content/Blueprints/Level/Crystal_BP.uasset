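; Collectible crystal pickup that can patrol back and forth along the world X axis.
; While CanMove is set, Tick moves it by Speed without sweeping and reverses direction at plus or minus MaxX, measured from the world origin rather than its start point.
; On overlap with GameCharacter_FirstUnrealGame, it increments that character's CrystalCount and destroys itself.
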(event `self.ReceiveTick`
  (params (DeltaSeconds :type "Float (single-precision)"))
  (bind _returnvalue_x (`KismetMathLibrary.BreakVector` (`self.K2_GetActorLocation`)))
  (bind (_returnvalue_x_2 _returnvalue_y _returnvalue_z) (`KismetMathLibrary.BreakVector` (`self.K2_GetActorLocation`)))
  (bind _returnvalue_x_3 (`KismetMathLibrary.BreakVector` (`self.K2_GetActorLocation`)))
  (if (`self.Can Move`)
    (`self.K2_SetActorLocation` (`KismetMathLibrary.MakeVector` (+ _returnvalue_x_2 (* (`self.Speed`) DeltaSeconds)) _returnvalue_y _returnvalue_z))
    (if (>= _returnvalue_x_3 (`self.Max X`))
      (set `self.Speed` (* (`self.Speed`) -1.0))
      (elif (<= _returnvalue_x (* (`self.Max X`) -1.0))
        (set `self.Speed` (`KismetMathLibrary.Abs` (`self.Speed`)))))))

(event `self.ReceiveActorBeginOverlap`
  (params (OtherActor :type "Actor Object Reference"))
  (bind _asgame_character_first_unreal_game (cast `/Game/Blueprints/GameCharacter_FirstUnrealGame` OtherActor))
  (`/Engine/EditorBlueprintResources/StandardMacros.IncrementInt` (`/Game/Blueprints/GameCharacter_FirstUnrealGame.Crystal Count` _asgame_character_first_unreal_game)
    (:`  `
      (`self.K2_DestroyActor`))))

(fn `UserConstructionScript`)