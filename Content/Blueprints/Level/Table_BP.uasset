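; Table Blueprint that tracks whether a chair is placed at the table.
; When a Chair_BP begins or ends overlap with TableCollision, it sets ChairInPlace true or false on the player's GameCharacter_FirstUnrealGame.
; Each change also prints the new value on screen as debug output.
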(event `self.Table Collision.OnComponentBeginOverlap`
  (params (OverlappedComponent :type "PrimitiveComponent Object Reference") (OtherActor :type "Actor Object Reference") (OtherComp :type "PrimitiveComponent Object Reference") (OtherBodyIndex :type Integer) (bFromSweep :type Boolean) (SweepResult :type "HitResult Structure (by ref)"))
  (cast `/Game/Blueprints/Level/Chair_BP` OtherActor)
  (bind _asgame_character_first_unreal_game (cast `/Game/Blueprints/GameCharacter_FirstUnrealGame` (`GameplayStatics.GetPlayerCharacter` 0)))
  (bind _output_get (set `/Game/Blueprints/GameCharacter_FirstUnrealGame.ChairInPlace` true _asgame_character_first_unreal_game))
  (`KismetSystemLibrary.PrintString` (`KismetStringLibrary.Conv_BoolToString` _output_get)))

(event `self.Table Collision.OnComponentEndOverlap`
  (params (OverlappedComponent :type "PrimitiveComponent Object Reference") (OtherActor :type "Actor Object Reference") (OtherComp :type "PrimitiveComponent Object Reference") (OtherBodyIndex :type Integer))
  (cast `/Game/Blueprints/Level/Chair_BP` OtherActor)
  (bind _asgame_character_first_unreal_game (cast `/Game/Blueprints/GameCharacter_FirstUnrealGame` (`GameplayStatics.GetPlayerCharacter` 0)))
  (bind _output_get (set `/Game/Blueprints/GameCharacter_FirstUnrealGame.ChairInPlace` false _asgame_character_first_unreal_game))
  (`KismetSystemLibrary.PrintString` (`KismetStringLibrary.Conv_BoolToString` _output_get)))

(fn `UserConstructionScript`)